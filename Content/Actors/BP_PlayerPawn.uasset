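; Player ship pawn for a shooter played in the Y-Z plane under an orthographic camera.
; Enhanced Input sets a target velocity that Tick eases toward with separate acceleration and deceleration, while smoothly tilting the mesh from input.
; Position is clamped to bounds cached from the view-target camera's ortho width and viewport aspect, pairing ship Y with camera Z and vice versa.
; Shooting is rate-limited, with WeaponLevel selecting single, parallel double or three-way spread bullets.
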(event Input|EnhancedActionEvents|EnhancedInputActionIA_Move
  (params (ActionValue :type Vector%202D%20Structure) (ElapsedSeconds :type Float%20%28double-precision%29) (TriggeredSeconds :type Float%20%28double-precision%29) (InputAction :type Input%20Action%20Object%20Reference :default "/Game/Game/IA_Move.IA_Move"))
  (bind (_x _y) (Math|Vector2D|BreakVector2D ActionValue))
  (:Triggered
    (bind _output_get (Variables|Default|SetTargetVelocity (* (Math|Vector|Normalize (Math|Vector|MakeVector 0.0 _x _y)) (Variables|Default|GetMoveSpeed)))))
  (:Completed
    (Variables|Default|SetTargetVelocity "0, 0, 0")))

(event Input|EnhancedActionEvents|EnhancedInputActionIA_Shoot
  (params (ActionValue :type Boolean) (ElapsedSeconds :type Float%20%28double-precision%29) (TriggeredSeconds :type Float%20%28double-precision%29) (InputAction :type Input%20Action%20Object%20Reference :default "/Game/Game/IA_Shoot.IA_Shoot"))
  (bind _returnvalue (Utilities|Time|GetGameTimeinSeconds))
  (bind _bulletspawn (Variables|Default|GetBulletSpawn))
  (bind _returnvalue_2 (Transformation|GetWorldTransform _bulletspawn))
  (bind (_location _rotation _scale) (Math|Transform|BreakTransform _returnvalue_2))
  (if (>= (- _returnvalue (Variables|Default|GetLastFireTime)) (Variables|Default|GetFireRate))
    (switch int (Variables|Default|GetWeaponLevel)
      (:1
        (Game|SpawnActorfromClass "/Game/Actors/BP_Bullet.BP_Bullet_C" _returnvalue_2 "Undefined" "MultiplyWithRoot" 0 0))
      (:2
        (Game|SpawnActorfromClass "/Game/Actors/BP_Bullet.BP_Bullet_C" (Math|Transform|MakeTransform (+ _location (Math|Vector|MakeVector 0.0 0.0 1e+02)) _rotation _scale) "Undefined" "MultiplyWithRoot" 0 0)
        (Game|SpawnActorfromClass "/Game/Actors/BP_Bullet.BP_Bullet_C" (Math|Transform|MakeTransform (+ _location (Math|Vector|MakeVector 0.0 0.0 -1e+02)) _rotation _scale) "Undefined" "MultiplyWithRoot" 0 0))
      (:3
        (Game|SpawnActorfromClass "/Game/Actors/BP_Bullet.BP_Bullet_C" _returnvalue_2 "Undefined" "MultiplyWithRoot" 0 0)
        (bind _returnvalue_3 (Game|SpawnActorfromClass "/Game/Actors/BP_Bullet.BP_Bullet_C" _returnvalue_2 "Undefined" "MultiplyWithRoot" 0 0))
        (Variables|/Game/Actors/BP_Bullet.BP_Bullet_C|SetDirection _returnvalue_3 "0.000000,1.000000,0.500000")
        (bind _returnvalue_4 (Game|SpawnActorfromClass "/Game/Actors/BP_Bullet.BP_Bullet_C" _returnvalue_2 "Undefined" "MultiplyWithRoot" 0 0))
        (Variables|/Game/Actors/BP_Bullet.BP_Bullet_C|SetDirection _returnvalue_4 "0.000000,1.000000,-0.500000")))
    (Variables|Default|SetLastFireTime _returnvalue)))

(event EventBeginPlay
  (bind _returnvalue (Game|GetPlayerController 0))
  (bind _returnvalue_2 (Viewport|GetViewportSize))
  (bind (_x _y) (Math|Vector2D|BreakVector2D _returnvalue_2))
  (Input|AddMappingContext (PlayerController|LocalPlayerSubsystems|GetEnhancedInputLocalPlayerSubsystem _returnvalue) "/Game/Game/IMC_Player.IMC_Player" 1 "(bIgnoreAllPressedKeysUntilRelease=True,bForceImmediately=False,bNotifyUserSettings=False)")
  (bind _ascamera_actor (Utilities|Casting|CastToCameraActor (Pawn|GetViewTarget _returnvalue)))
  (bind _output_get (Variables|Default|SetGameCamera _ascamera_actor))
  (Variables|Default|SetCameraHalfWidth (/ (/ (Variables|/Script/Engine.CameraComponent|GetOrthoWidth (Variables|/Script/Engine.CameraActor|GetCameraComponent _output_get)) 2.0) (/ _x _y)))
  (Variables|Default|SetCameraHalfHeight (/ (Variables|/Script/Engine.CameraComponent|GetOrthoWidth (Variables|/Script/Engine.CameraActor|GetCameraComponent _output_get)) 2.0)))

(event Collision|EventActorBeginOverlap
  (params (OtherActor :type Actor%20Object%20Reference)))

(event EventTick
  (params (DeltaSeconds :type Float%20%28single-precision%29))
  (bind _returnvalue (Transformation|GetActorLocation))
  (bind _returnvalue_2 (Utilities|Time|GetWorldDeltaSeconds))
  (bind _gamecamera (Variables|Default|GetGameCamera))
  (bind _camerahalfwidth (Variables|Default|GetCameraHalfWidth))
  (bind _shipradius (Variables|Default|GetShipRadius))
  (bind _camerahalfheight (Variables|Default|GetCameraHalfHeight))
  (bind _gamecamera_2 (Variables|Default|GetGameCamera))
  (bind _shipradius_2 (Variables|Default|GetShipRadius))
  (bind (_x _y _z) (Math|Vector|BreakVector _returnvalue))
  (bind _returnvalue_3 (Transformation|GetActorLocation _gamecamera_2))
  (bind _returnvalue_4 (Transformation|GetActorLocation _gamecamera))
  (bind _z_2 (Math|Vector|BreakVector _returnvalue_3))
  (bind _y_2 (Math|Vector|BreakVector _returnvalue_4))
  (bind _output_get (Variables|Default|SetCurrentVelocity (Math|Interpolation|VInterpTo (Variables|Default|GetCurrentVelocity) (stale Input|EnhancedActionEvents|EnhancedInputActionIA_Move _output_get) DeltaSeconds (Math|Float|SelectFloat (Variables|Default|GetAcceleration) (Variables|Default|GetDeceleration) (> (Math|Vector|VectorLength (stale Input|EnhancedActionEvents|EnhancedInputActionIA_Move _output_get)) 5.0)))))
  (Transformation|AddActorWorldOffset (* _output_get DeltaSeconds))
  (Transformation|SetActorLocation (Math|Vector|MakeVector _x (Math|Float|Clamp(Float) _y (+ (- _z_2 _camerahalfheight) _shipradius_2) (- (+ _z_2 _camerahalfheight) _shipradius_2)) (Math|Float|Clamp(Float) _z (+ (- _y_2 _camerahalfwidth) _shipradius) (- (+ _y_2 _camerahalfwidth) _shipradius))) false false)
  (bind _output_get_2 (Variables|Default|SetCurrentRoll (Math|Interpolation|FInterpTo (Variables|Default|GetCurrentRoll) (* (* (.Y (Math|Vector2D|BreakVector2D (stale Input|EnhancedActionEvents|EnhancedInputActionIA_Move ActionValue))) (Variables|Default|GetMaxRollAngle)) -1.0) _returnvalue_2 (Variables|Default|GetRollInterpSpeed))))
  (bind _output_get_3 (Variables|Default|SetCurrentPitch (Math|Interpolation|FInterpTo (Variables|Default|GetCurrentPitch) (* (* (Variables|Default|GetMaxPitchangle) (.X (Math|Vector2D|BreakVector2D (stale Input|EnhancedActionEvents|EnhancedInputActionIA_Move ActionValue)))) 1.0) _returnvalue_2 (Variables|Default|GetPitchInterpSpeed))))
  (Transformation|SetRelativeRotation (Variables|Default|GetStaticMeshComponent0) (Math|Rotator|MakeRotator _output_get_2 _output_get_3 9e+01) false false))

(fn ConstructionScript)