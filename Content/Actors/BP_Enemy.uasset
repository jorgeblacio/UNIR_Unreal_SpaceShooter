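; BP_Enemy is a shootable enemy actor that travels along negative Y at its move speed.
; On BeginPlay it moves to Y equal to the viewport width at a random Z within the viewport height, treating pixels as world units, and sets a limited lifespan.
; Each overlapping BP_Bullet removes one hit point.
; The killing hit plays a sound and destroys both actors; earlier hits leave the bullet alive.
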(event EventBeginPlay
  (bind _returnvalue (Transformation|GetActorTransform))
  (bind _returnvalue_2 (Viewport|GetViewportSize))
  (bind (_location _rotation _scale) (Math|Transform|BreakTransform _returnvalue))
  (bind (_x _y) (Math|Vector2D|BreakVector2D _returnvalue_2))
  (bind _returnvalue_3 (/ _y 2.0))
  (Transformation|SetActorTransform (Math|Transform|MakeTransform (Math|Vector|MakeVector (.X (Math|Vector|BreakVector _location)) _x (Math|Random|RandomFloatinRange (* _returnvalue_3 -1.0) _returnvalue_3)) _rotation _scale))
  (Actor|SetLifeSpan (Variables|Default|GetLifeTime)))

(event Collision|EventActorBeginOverlap
  (params (OtherActor :type Actor%20Object%20Reference))
  (bind _asbp_bullet (Utilities|Casting|CastToBP_Bullet OtherActor))
  (Utilities|IsValid _asbp_bullet
    (:Is%20Valid
      (bind _output_get (Variables|Default|SetHitPoints (- (Variables|Default|GetHitPoints) 1.0)))
      (if (<= _output_get 0.0)
        (Audio|PlaySound2D "/Game/Free_Sounds_Pack/cue/Wood_Move_2-1_Cue.Wood_Move_2-1_Cue" 1.0 1.0 0.0 0 0)
        (Actor|DestroyActor)
        (Actor|DestroyActor _asbp_bullet)))))

(event EventTick
  (params (DeltaSeconds :type Float%20%28single-precision%29))
  (Transformation|AddActorWorldOffset (Math|Vector|MakeVector 0.0 (* (* (Variables|Default|GetMoveSpeed) -1.0) DeltaSeconds) 0.0)))

(fn ConstructionScript)